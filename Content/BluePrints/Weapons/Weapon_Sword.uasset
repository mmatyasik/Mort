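; Physics-driven sword weapon that damages Enemy actors it overlaps, scaled by how fast it is moving.
; On overlap it rewinds the Blood flipbook to its first frame and applies damage proportional to the Capsule's velocity.
; It also spikes the Capsule's linear damping so the blade drags inside the enemy, then clears it when the overlap ends.
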(event EventBeginPlay)

(event EventTick
  (params (DeltaSeconds :type Float%20%28single-precision%29)))

(event Collision|EventActorBeginOverlap
  (params (OtherActor :type Actor%20Object%20Reference))
  (if (Utilities|ClassIsChildOf (Utilities|GetClass OtherActor) "/Game/BluePrints/Enemy/Enemy.Enemy_C")
    (Class|PrimitiveComponent|SetLinearDamping (Variables|Default|GetCapsule) 6e+03)
    (Class|PaperFlipbookComponent|SetPlaybackPositioninFrames (Variables|Default|GetBlood) 0 false)
    (Game|Damage|ApplyDamage OtherActor (/ (Math|Vector|VectorLength (Transformation|GetComponentVelocity (Variables|Default|GetCapsule))) 7.0) 0 self)))

(event Collision|EventActorEndOverlap
  (params (OtherActor :type Actor%20Object%20Reference))
  (if (Utilities|ClassIsChildOf (Utilities|GetClass OtherActor) "/Game/BluePrints/Enemy/Enemy.Enemy_C")
    (Class|PrimitiveComponent|SetLinearDamping (Variables|Default|GetCapsule) 0.0)))

(fn ConstructionScript
  (|CallParentFunction))