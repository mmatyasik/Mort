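; Gate bomb spell, a flipbook-animated child spell that costs mana and deals no damage.
; Each tick it checks the physics capsule's speed, and once nearly stopped it marks itself dead, disables physics, switches collision to overlap-all and resizes the capsule.
; Its animation update shows an explosion flipbook for a second, then the idle or dead flipbook chosen by a simple state selector.
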(event EventBeginPlay)

(event Collision|EventActorBeginOverlap
  (params (OtherActor :type Actor%20Object%20Reference)))

(event EventTick
  (params (DeltaSeconds :type Float%20%28single-precision%29))
  (bind _capsule (Variables|Default|GetCapsule))
  (if (and (<= (Math|Vector|VectorLength (Transformation|GetComponentVelocity (Variables|Default|GetCapsule))) 15.0) (not (Variables|Default|GetDead?)))
    (Variables|Default|SetDead? true)
    (CallFunction|UpdateAnimation)
    (Physics|SetSimulatePhysics _capsule false)
    (Collision|SetCollisionProfileName _capsule "OverlapAll" :!class /Script/Engine.PrimitiveComponent)
    (Components|Capsule|SetCapsuleSize (Variables|Default|GetCapsule) 14.0 14.0 true)))

(fn ConstructionScript
  (|CallParentFunction)
  (Variables|Default|SetMana_cost 1e+02)
  (Variables|Default|SetDamage 0.0))

(fn AnimStateMachine
  (params (Dead? :type Boolean))
  (if Dead?
    (Variables|Default|SetAnimationState "NewEnumerator1")
    (else
      (Variables|Default|SetAnimationState "NewEnumerator0")))
  (return (Utilities|Select :Index (Variables|Default|GetAnimationState) :NewEnumerator1 (Variables|Default|GetDead%20Flipbook) :NewEnumerator0 (Variables|Default|GetIdle%20Flipbook))))

(event Custom|UpdateAnimation
  (bind _currentflipbook (CallFunction|AnimStateMachine (Variables|Default|Getdead?)))
  (Sprite|SetFlipbook (Variables|Default|GetFlipBook) "/Game/Art/Sprites/Flipbooks/explosion.explosion")
  (Utilities|FlowControl|Delay 1.0)
  (Sprite|SetFlipbook (Variables|Default|GetFlipBook) _currentflipbook)
  (return))