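; Player pawn: a physics-driven character with swappable melee weapons, a mana-gated spell, pickups and a life/mana HUD.
; Tick pushes the capsule with input forces, disabling CharacterMovement, and steers the weapon's constraint joint toward the mouse while left-click is held.
; Collisions deal self-damage scaled by relative velocity, with brief invulnerability afterwards.
; Touching a bomb gate plays an explosion then loads Level_2; J/K/L are stat debug keys.
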(event Collision|EventActorBeginOverlap
  (params (OtherActor :type Actor%20Object%20Reference))
  (if (== (Utilities|GetClass OtherActor) "/Game/BluePrints/Spell/Spell_Bomb_Gate.Spell_Bomb_Gate_C")
    (Development|PrintString "GATE !!!!")
    (bind _asspell_bomb_gate (Utilities|Casting|CastToSpell_Bomb_Gate OtherActor))
    (Sprite|SetFlipbook (Variables|/Game/BluePrints/Spell/Spell.Spell_C|GetFlipBook _asspell_bomb_gate) "/Game/Art/Sprites/Flipbooks/explosion.explosion")
    (Utilities|FlowControl|Delay 1.0)
    (Sprite|SetFlipbook (Variables|/Game/BluePrints/Spell/Spell.Spell_C|GetFlipBook _asspell_bomb_gate) "/Game/Art/Sprites/Flipbooks/HeroFlipbook.HeroFlipbook")
    (Game|OpenLevel(byName) "Level_2")
    (Development|PrintString "BRAVVVOOO")))

(event EventBeginPlay
  (CallFunction|CreateHUD)
  (Variables|/Script/Engine.PlayerController|SetbShowMouseCursor (Game|GetPlayerController 0) true)
  (|SetPhysicsConstraint(Spring)))

(event EventTick
  (params (DeltaSeconds :type Float%20%28single-precision%29))
  (|CharacterWalk)
  (Pawn|Components|CharacterMovement|SetMovementMode (Variables|Character|GetCharacterMovement) "MOVE_None" 0)
  (|SetSliderValues)
  (if (Game|Player|IsInputKeyDown (Game|GetPlayerController 0) "LeftMouseButton")
    (|RotateTheSword :!label _label)
    (else
      (goto _label false))))

(event Collision|EventHit
  (params (MyComp :type Primitive%20Component%20Object%20Reference) (Other :type Actor%20Object%20Reference) (OtherComp :type Primitive%20Component%20Object%20Reference) (bSelfMoved :type Boolean) (HitLocation :type Vector :default "0, 0, 0") (HitNormal :type Vector :default "0, 0, 0") (NormalImpulse :type Vector :default "0, 0, 0") (Hit :type Hit%20Result%20Structure%20%28by%20ref%29))
  (bind _returnvalue (Transformation|GetVelocity Other))
  (bind _returnvalue_2 (Transformation|GetVelocity))
  (bind _returnvalue_3 (- _returnvalue _returnvalue_2))
  (bind _returnvalue_4 (Math|Vector|VectorLength _returnvalue_3))
  (if (> _returnvalue_4 2e+01)
    (Game|Damage|ApplyDamage self (/ _returnvalue_4 1.8e+02) 0 Other "/Engine/EngineDamageTypes/DmgTypeBP_Environmental.DmgTypeBP_Environmental_C")))

(event Game|Damage|EventAnyDamage
  (params (Damage :type Float%20%28single-precision%29) (DamageType :type Damage%20Type%20Object%20Reference) (InstigatedBy :type Controller%20Object%20Reference) (DamageCauser :type Actor%20Object%20Reference))
  (Variables|Default|Setlife (- (Variables|Current|GetLife) Damage))
  (Audio|PlaySoundatLocation "/Game/Art/Sounds/PlayerPain1.PlayerPain1" (Transformation|GetWorldLocation (Variables|Collision|GetCapsuleComponent)) "0, 0, 0" 1.0 0.85 0.0 0 "/Game/Art/Sounds/SoundConcurency.SoundConcurency")
  (Variables|Actor|SetbCanBeDamaged false)
  (Utilities|FlowControl|Delay 0.2)
  (Variables|Actor|SetbCanBeDamaged true))

(event Input|ActionEvents|InputActionSword
  (params (Key :type Key%20Structure :default "AnyKey"))
  (:Pressed
    (ChildActorComponent|SetChildActorClass (Variables|Default|GetWeapon%20Slot) "/Game/BluePrints/Weapons/Weapon_Sword.Weapon_Sword_C")
    (|SetPhysicsConstraint(Spring))))

(event Input|ActionEvents|InputActionAxe
  (params (Key :type Key%20Structure :default "AnyKey"))
  (:Pressed
    (ChildActorComponent|SetChildActorClass (Variables|Default|GetWeapon%20Slot) "/Game/BluePrints/Weapons/Weapon_Axe.Weapon_Axe_C")
    (|SetPhysicsConstraint(Spring))))

(event Input|ActionEvents|InputActionMace
  (params (Key :type Key%20Structure :default "AnyKey"))
  (:Pressed
    (ChildActorComponent|SetChildActorClass (Variables|Default|GetWeapon%20Slot) "/Game/BluePrints/Weapons/Weapon_Mace.Weapon_Mace_C")
    (|SetPhysicsConstraint(Spring))))

(event Input|ActionEvents|InputActionSpell
  (params (Key :type Key%20Structure :default "AnyKey"))
  (:Pressed
    (if (>= (Variables|Current|GetMana) (Variables|Stats|GetMaxMana))
      (Variables|Current|SetMana (- (Variables|Current|GetMana) 1e+02))
      (|ShootGATE))))

(event Input|KeyboardEvents|L
  (params (Key :type Key%20Structure :default "AnyKey"))
  (:Pressed
    (Variables|Current|SetLife (+ (Variables|Current|GetLife) 1e+01))))

(event Input|KeyboardEvents|K
  (params (Key :type Key%20Structure :default "AnyKey"))
  (bind _life (Variables|Current|GetLife))
  (:Pressed
    (Math|Float|DecrementFloat _life
      (:%20%20
        (Math|Float|DecrementFloat _life
          (:%20%20
            (Math|Float|DecrementFloat (Variables|Current|GetLife))))))))

(event Input|KeyboardEvents|J
  (params (Key :type Key%20Structure :default "AnyKey"))
  (:Pressed
    (Variables|Current|SetMana (Variables|Stats|GetMaxMana))))

(fn ConstructionScript)

(fn Pick
  (params (pickable :type Pickable%20Object%20Reference))
  (bind _returnvalue (Utilities|GetClass pickable))
  (bind _returnvalue_2 (Utilities|GetClassDisplayName _returnvalue))
  (Development|PrintString _returnvalue_2)
  (switch name (Utilities|String|StringToName _returnvalue_2)
    (:Pickable_Soul_C
      (Variables|Current|SetMana (+ (Variables|Current|GetMana) 1e+01))
      (Math|Float|IncrementFloat (Variables|Current|GetSouls)))
    (:Pickable_Coin_C
      (Math|Integer|IncrementInt (Math|Float|Truncate (Variables|Current|GetGold))))))

(fn CreateHUD
  (bind _returnvalue (UserInterface|CreateWidget "/Game/BluePrints/GUI/playHUDwidget.PlayHUDwidget_C"))
  (bind _output_get (Variables|Hud|SetPlayHUDreference _returnvalue))
  (UserInterface|Viewport|AddtoViewport _output_get 0)
  (return))