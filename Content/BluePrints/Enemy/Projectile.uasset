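; Enemy projectile actor that damages the player on hit.
; A hit on a Weapon-derived actor destroys it, while a hit on PlayerBP applies its damage value to the player pawn without destroying it.
; Tick also destroys the projectile once its speed falls into a low, non-zero range, clearing out nearly stopped shots.
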(event EventBeginPlay)

(event Collision|EventActorBeginOverlap
  (params (OtherActor :type Actor%20Object%20Reference)))

(event Collision|EventHit
  (params (MyComp :type Primitive%20Component%20Object%20Reference) (Other :type Actor%20Object%20Reference) (OtherComp :type Primitive%20Component%20Object%20Reference) (bSelfMoved :type Boolean) (HitLocation :type Vector :default "0, 0, 0") (HitNormal :type Vector :default "0, 0, 0") (NormalImpulse :type Vector :default "0, 0, 0") (Hit :type Hit%20Result%20Structure%20%28by%20ref%29))
  (if (Utilities|ClassIsChildOf (Utilities|GetClass Other) "/Game/BluePrints/Weapons/Weapon.Weapon_C")
    (Actor|DestroyActor)
    (elif (== (Utilities|GetClass Other) "/Game/BluePrints/PlayerBP.PlayerBP_C")
      (Game|Damage|ApplyDamage (Game|Player|GetPlayerPawn 0) (Variables|Default|GetProjectileDamage) 0 self))))

(event EventTick
  (params (DeltaSeconds :type Float%20%28single-precision%29))
  (if (Math|Float|InRange(Float) (Math|Vector|VectorLength (Transformation|GetVelocity)) 1.0 2e+01)
    (Actor|DestroyActor)))

(fn ConstructionScript)