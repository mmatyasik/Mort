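; Paper2D flipbook enemy that chases the player by turning its capsule and applying force each Tick.
; Hard physics impacts deal damage scaled by impulse; damage plays blood and sound, with brief protection from further impacts.
; Weapon_Mace hits freeze its steering until a random per-tick roll releases it.
; When Life drops below zero it swaps to a dead flipbook, credits a player kill and is destroyed, dropping a soul pickup.
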(event Collision|EventHit
  (params (MyComp :type Primitive%20Component%20Object%20Reference) (Other :type Actor%20Object%20Reference) (OtherComp :type Primitive%20Component%20Object%20Reference) (bSelfMoved :type Boolean) (HitLocation :type Vector :default "0, 0, 0") (HitNormal :type Vector :default "0, 0, 0") (NormalImpulse :type Vector) (Hit :type Hit%20Result%20Structure%20%28by%20ref%29))
  (bind _returnvalue (Math|Vector|VectorLength NormalImpulse))
  (bind _returnvalue_2 (/ _returnvalue 5e+02))
  (if (> _returnvalue_2 6.0)
    (if (not (Variables|Default|Getindestructible?))
      (Development|PrintString (Utilities|String|ToString(Float) _returnvalue_2) true true "(R=0.000000,G=0.660000,B=1.000000,A=1.000000)" 2.0)
      (Game|Damage|ApplyDamage self _returnvalue_2 0 Other))))

(event EventTick
  (params (DeltaSeconds :type Float%20%28single-precision%29))
  (bind _returnvalue (Game|Player|GetPlayerPawn 0))
  (bind _capsule (Variables|Default|GetCapsule))
  (bind _returnvalue_2 (Transformation|GetActorLocation _returnvalue))
  (bind _relativelocation (Variables|/Script/Engine.SceneComponent|GetRelativeLocation _capsule))
  (bind _returnvalue_3 (Math|Rotator|FindLookatRotation _relativelocation _returnvalue_2))
  (bind _yaw (Math|Rotator|BreakRotator _returnvalue_3))
  (bind _returnvalue_4 (Math|Rotator|MakeRotator -9e+01 0.0 _yaw))
  (if (Variables|Default|Getfrozen?)
    (if (== (Math|Random|RandomIntegerinRange 0 1000) 0)
      (Variables|Default|Setfrozen? false)
      (Transformation|SetRelativeRotation _capsule _returnvalue_4 false false :!label _label)
      (Physics|AddForce (Variables|Default|GetCapsule) (* (Math|Vector|GetForwardVector _returnvalue_4) 1e+01) "None" true))
    (else
      (goto _label))))

(event Game|Damage|EventAnyDamage
  (params (Damage :type Float%20%28single-precision%29) (DamageType :type Damage%20Type%20Object%20Reference) (InstigatedBy :type Controller%20Object%20Reference) (DamageCauser :type Actor%20Object%20Reference))
  (Variables|Default|Setlife (- (Variables|Default|Getlife) Damage))
  (Components|Timeline|PlayfromStart (Variables|Default|GetBlood))
  (Audio|PlaySound2D "/Game/Art/Sounds/HIT.HIT" (Math|Random|RandomFloatinRange 1e+01 2e+01) (Math|Random|RandomFloatinRange 0.5 2.0) 0.0 "/Game/Art/Sounds/SoundConcurency.SoundConcurency")
  (Variables|Default|Setindestructible? true)
  (Utilities|FlowControl|Delay 0.1)
  (Variables|Default|Setindestructible? false)
  (|CheckDamageCauser DamageCauser)
  (|DEAD))

(event EventDestroyed
  (|DropLOOT_2))

(fn ConstructionScript
  (Components|Timeline|SetLooping (Variables|Default|GetBlood) false)
  (Audio|Components|Audio|Stop (Variables|Default|GetBlood)))

(fn AnimStateMachine
  (params (dead? :type Boolean))
  (if dead?
    (Variables|Animations|SetAnimationState "NewEnumerator1")
    (else
      (Variables|Animations|SetAnimationState "NewEnumerator0")))
  (return (Utilities|Select :Index (Variables|Animations|GetAnimationState) :NewEnumerator1 (Variables|Animations|GetDead%20Flipbook) :NewEnumerator0 (Variables|Animations|GetIdle%20Flipbook))))

(event Custom|UpdateAnimation
  (bind _currentflipbook (CallFunction|AnimStateMachine (Variables|Default|Getdead?)))
  (Sprite|SetFlipbook (Variables|Default|GetFlipBook) _currentflipbook))