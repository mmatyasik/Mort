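; Enemy_Ranged is an enemy Blueprint that randomly fires projectiles in the direction it faces.
; BeginPlay runs the parent logic, then sets the death flipbook to Explosion and the projectile type to Projectile.
; Each Tick has roughly a 1-in-1000 chance to spawn a projectile at the actor's location with its capsule's rotation and push it forward with a physics impulse, so fire rate depends on frame rate.
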(event EventBeginPlay
  (|CallParentFunction)
  (Variables|Default|SetDead%20Flipbook "/Game/Art/Sprites/Flipbooks/explosion.explosion")
  (Variables|Default|SetProjectile%20Type "/Game/BluePrints/Enemy/Projectile.Projectile_C"))

(event EventTick
  (params (DeltaSeconds :type Float%20%28single-precision%29))
  (bind _capsule (Variables|Default|GetCapsule))
  (bind _returnvalue (Transformation|GetWorldRotation _capsule))
  (|CallParentFunction 0.0)
  (if (== (Math|Random|RandomIntegerinRange 0 1000) 0)
    (bind _returnvalue_2 (Game|SpawnActorfromClass (Variables|Default|GetProjectile%20Type) (Math|Transform|MakeTransform (Transformation|GetActorLocation) _returnvalue) "AdjustIfPossibleButAlwaysSpawn" 0 0))
    (bind _asprojectile (Utilities|Casting|CastToProjectile _returnvalue_2))
    (Physics|AddImpulse (Variables|/Game/BluePrints/Enemy/Projectile.Projectile_C|GetCapsule _asprojectile) (* (Math|Vector|GetForwardVector _returnvalue) 1e+02) "None" false)))

(fn ConstructionScript
  (|CallParentFunction))